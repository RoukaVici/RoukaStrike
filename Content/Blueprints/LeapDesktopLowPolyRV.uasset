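; LeapDesktopLowPolyRV is a Leap Motion hands Blueprint that shows tracked left and right hands and tracks objects they could pick up.
; On BeginPlay it scales OffsetAndScale by world-to-meters so hand size stays constant.
; Leap visibility events show or hide each hand.
; Each hand's collider caches an overlapping PIckupInterface actor and clears it on exit; no grab or drop logic appears here.
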(event OnLeftHandVisibilityChanged(Leap)
  (params (bIsVisible :type Boolean))
  (bind _left (Variables|Default|GetLeft))
  (if bIsVisible
    (Development|SetHiddeninGame _left false false)
    (else
      (Development|SetHiddeninGame _left true false))))

(event OnRightHandVisibilityChanged(Leap)
  (params (bIsVisible :type Boolean))
  (bind _right (Variables|Default|GetRight))
  (if bIsVisible
    (Development|SetHiddeninGame _right false false)
    (else
      (Development|SetHiddeninGame _right true false))))

(event EventBeginPlay
  (Transformation|SetRelativeScale3D (Variables|Default|GetOffsetAndScale) (Math|Conversions|ToVector(Float) (/ (Class|HeadMountedDisplayFunctionLibrary|GetWorldtoMetersScale) 1e+02))) ; Hands are always same size
)

(event OnComponentBeginOverlap(LeftCollider)
  (params (OverlappedComponent :type Primitive%20Component%20Object%20Reference) (OtherActor :type Actor%20Object%20Reference) (OtherComp :type Primitive%20Component%20Object%20Reference) (OtherBodyIndex :type Integer) (bFromSweep :type Boolean) (SweepResult :type Hit%20Result%20Structure%20%28by%20ref%29))
  (if (Utilities|DoesObjectImplementInterface OtherActor "/Game/Blueprints/PIckupInterface.PIckupInterface_C")
    (Variables|Default|SetLeftOverlapActor OtherActor)))

(event OnComponentBeginOverlap(RightCollider)
  (params (OverlappedComponent :type Primitive%20Component%20Object%20Reference) (OtherActor :type Actor%20Object%20Reference) (OtherComp :type Primitive%20Component%20Object%20Reference) (OtherBodyIndex :type Integer) (bFromSweep :type Boolean) (SweepResult :type Hit%20Result%20Structure%20%28by%20ref%29))
  (if (Utilities|DoesObjectImplementInterface OtherActor "/Game/Blueprints/PIckupInterface.PIckupInterface_C")
    (Variables|Default|SetRightOverlapActor OtherActor)))

(event OnComponentEndOverlap(LeftCollider)
  (params (OverlappedComponent :type Primitive%20Component%20Object%20Reference) (OtherActor :type Actor%20Object%20Reference) (OtherComp :type Primitive%20Component%20Object%20Reference) (OtherBodyIndex :type Integer))
  (if (== OtherActor (Variables|Default|GetLeftOverlapActor))
    (Variables|Default|SetLeftOverlapActor 0)))

(event OnComponentEndOverlap(RightCollider)
  (params (OverlappedComponent :type Primitive%20Component%20Object%20Reference) (OtherActor :type Actor%20Object%20Reference) (OtherComp :type Primitive%20Component%20Object%20Reference) (OtherBodyIndex :type Integer))
  (if (== OtherActor (Variables|Default|GetRightOverlapActor))
    (Variables|Default|SetRightOverlapActor 0)))

(fn ConstructionScript)