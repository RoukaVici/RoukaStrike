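; Leap Motion low-poly hands Blueprint for desktop mode, letting the player grab and release objects with either hand.
; BeginPlay scales the hands by world-to-meters and sets desktop tracking, EndPlay restores VR mode, and visibility events show or hide each hand.
; Per-hand colliders track an overlapping PIckupInterface actor.
; Grab and release events send it pickup and drop messages with that hand's component and handle.
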(event OnLeftHandVisibilityChanged(Leap)
  (params (bIsVisible :type Boolean))
  (bind _left (Variables|Default|GetLeft))
  (if bIsVisible
    (Development|SetHiddeninGame _left false true)
    (else
      (Development|SetHiddeninGame _left true true))))

(event OnRightHandVisibilityChanged(Leap)
  (params (bIsVisible :type Boolean))
  (bind _right (Variables|Default|GetRight))
  (if bIsVisible
    (Development|SetHiddeninGame _right false true)
    (else
      (Development|SetHiddeninGame _right true true))))

(event EventBeginPlay
  (Transformation|SetRelativeScale3D (Variables|Default|GetOffsetAndScale) (Math|Conversions|ToVector(Float) (/ (Class|HeadMountedDisplayFunctionLibrary|GetWorldtoMetersScale) 1e+02))) ; Hands are always same size
  (Class|LeapBlueprintFunctionLibrary|SetLeapMode "LEAP_MODE_DESKTOP" "LEAP_NORMAL"))

(event EventEndPlay
  (params (EndPlayReason :type EEndPlayReason%20Enum :default "Destroyed"))
  (Class|LeapBlueprintFunctionLibrary|SetLeapMode "LEAP_MODE_VR" "LEAP_NORMAL"))

(event OnHandGrabbed(Leap)
  (params (Hand :type Leap%20Hand%20Data%20Structure%20%28by%20ref%29))
  (if (Utilities|Enum|Equal(Enum) (.HandType (Utilities|Struct|BreakLeapHandData Hand)) "LEAP_HAND_RIGHT")
    (if (!= (Variables|Default|GetRightOverlapActor) 0)
      (bind _output_get (Variables|Default|SetRightHeldActor (Variables|Default|GetRightOverlapActor)))
      (Class|PIckupInterface|Pickup(Message) _output_get (Variables|Default|GetRight%20Collider) (Variables|Default|GetRightHandle)))
    (elif (!= (Variables|Default|GetLeftOverlapActor) 0)
      (bind _output_get_2 (Variables|Default|SetLeftHeldActor (Variables|Default|GetLeftOverlapActor)))
      (Class|PIckupInterface|Pickup(Message) _output_get_2 (Variables|Default|GetLeft%20Collider) (Variables|Default|GetLeftHandle)))))

(event OnComponentBeginOverlap(LeftCollider)
  (params (OverlappedComponent :type Primitive%20Component%20Object%20Reference) (OtherActor :type Actor%20Object%20Reference) (OtherComp :type Primitive%20Component%20Object%20Reference) (OtherBodyIndex :type Integer) (bFromSweep :type Boolean) (SweepResult :type Hit%20Result%20Structure%20%28by%20ref%29))
  (if (Utilities|DoesObjectImplementInterface OtherActor "/Game/Blueprints/PIckupInterface.PIckupInterface_C")
    (Variables|Default|SetLeftOverlapActor OtherActor)))

(event OnComponentBeginOverlap(RightCollider)
  (params (OverlappedComponent :type Primitive%20Component%20Object%20Reference) (OtherActor :type Actor%20Object%20Reference) (OtherComp :type Primitive%20Component%20Object%20Reference) (OtherBodyIndex :type Integer) (bFromSweep :type Boolean) (SweepResult :type Hit%20Result%20Structure%20%28by%20ref%29))
  (if (Utilities|DoesObjectImplementInterface OtherActor "/Game/Blueprints/PIckupInterface.PIckupInterface_C")
    (Variables|Default|SetRightOverlapActor OtherActor)))

(event OnComponentEndOverlap(LeftCollider)
  (params (OverlappedComponent :type Primitive%20Component%20Object%20Reference) (OtherActor :type Actor%20Object%20Reference) (OtherComp :type Primitive%20Component%20Object%20Reference) (OtherBodyIndex :type Integer))
  (if (== OtherActor (Variables|Default|GetLeftOverlapActor))
    (Variables|Default|SetLeftOverlapActor 0)))

(event OnComponentEndOverlap(RightCollider)
  (params (OverlappedComponent :type Primitive%20Component%20Object%20Reference) (OtherActor :type Actor%20Object%20Reference) (OtherComp :type Primitive%20Component%20Object%20Reference) (OtherBodyIndex :type Integer))
  (if (== OtherActor (Variables|Default|GetRightOverlapActor))
    (Variables|Default|SetRightOverlapActor 0)))

(event OnHandReleased(Leap)
  (params (Hand :type Leap%20Hand%20Data%20Structure%20%28by%20ref%29))
  (if (Utilities|Enum|Equal(Enum) (.HandType (Utilities|Struct|BreakLeapHandData Hand)) "LEAP_HAND_RIGHT")
    (if (!= (Variables|Default|GetRightHeldActor) 0)
      (Class|PIckupInterface|Drop(Message) (Variables|Default|GetRightHeldActor) (Variables|Default|GetRight) (Variables|Default|GetRightHandle))
      (Variables|Default|SetRightHeldActor 0))
    (elif (!= (Variables|Default|GetLeftHeldActor) 0)
      (Class|PIckupInterface|Drop(Message) (Variables|Default|GetLeftHeldActor) (Variables|Default|GetLeft) (Variables|Default|GetLeftHandle))
      (Variables|Default|SetLeftHeldActor 0))))

(fn ConstructionScript)